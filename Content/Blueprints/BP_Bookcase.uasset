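; BP_Bookcase is a bookcase actor that slides horizontally to a target location when its move event is called.
; The event plays a world camera shake at the bookcase, then runs the Movement timeline.
; Each update lerps the root's current X and Y toward TargetLocation using separate timeline vector channels, leaving Z unchanged.
; Because the lerp starts from the current position rather than a cached start, the motion compounds over updates.
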(event Custom|move
  (bind _targetlocation (Variables|Default|GetTargetLocation))
  (bind _sharedroot (Variables|Default|GetSharedRoot))
  (bind _returnvalue (Transformation|GetWorldLocation _sharedroot))
  (Camera|PlayWorldCameraShake "/Game/Blueprints/BP_CameraShake.BP_CameraShake_C" (Transformation|GetWorldLocation (Variables|Default|GetSharedRoot)) 0.0 5e+02)
  (bind _movementvalue (Timeline|Movement Play)
    (:Update
      (Transformation|SetWorldLocation (Variables|Default|GetSharedRoot) (Math|Vector|MakeVector (Math|Float|Lerp (.x _returnvalue) (.x _targetlocation) (.x _movementvalue)) (Math|Float|Lerp (.y _returnvalue) (.y _targetlocation) (.y _movementvalue)) (.z _returnvalue)) false false))))

(fn ConstructionScript)