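; Double door Blueprint that swings two door meshes open and closed when interacted with.
; BeginPlay caches both doors' relative rotations as the closed pose.
; Interact, ignored while IsClosed is true, flip-flops between playing and reversing a Timeline.
; The Timeline track scales separate Rota and Rota0 angles added to each door's cached yaw.
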(event EventInteract
  (bind _rota_door_1 (Variables|Default|Getrota%20door%201))
  (bind _rota_door_2 (Variables|Default|Getrota%20door%202))
  (if (not (Variables|Default|Getis%20closed))
    (Utilities|FlowControl|FlipFlop
      (:A
        (bind _newtrack_0 (Timeline|Timeline Play)
          (:Update
            (Transformation|SetRelativeRotation (Variables|Default|GetDoor_1_StaticMeshComponent0) (Math|Rotator|MakeRotator (.roll _rota_door_1) (.pitch _rota_door_1) (+ (.yaw _rota_door_1) (* _newtrack_0 (Variables|Default|Getrota)))) false false)
            (Transformation|SetRelativeRotation (Variables|Default|GetDoor_2_StaticMeshComponent0) (Math|Rotator|MakeRotator (.roll _rota_door_2) (.pitch _rota_door_2) (+ (* _newtrack_0 (Variables|Default|Getrota_0)) (.yaw _rota_door_2))) false false))))
      (:B
        (Timeline|Timeline Reverse)))))

(event EventBeginPlay
  (Variables|Default|Setrota%20door%201 (Variables|/Script/Engine.SceneComponent|GetRelativeRotation (Variables|Default|GetDoor_1_StaticMeshComponent0)))
  (Variables|Default|Setrota%20door%202 (Variables|/Script/Engine.SceneComponent|GetRelativeRotation (Variables|Default|GetDoor_2_StaticMeshComponent0))))

(fn ConstructionScript)